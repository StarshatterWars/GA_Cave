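; Bot_Spikes is an armed bot that fires projectiles at found enemies and handles its own death.
; On BeginPlay it spawns a rifle on the WeaponPoint socket and binds a noise-hearing handler, which is empty.
; EnemyFound_Event spawns projectiles from the rifle with a yaw offset and sound, rate-limited by a DoOnce reset after a short delay.
; BotDeath_Event clears Alive, plays the death animation, then calls the BotHasDied dispatcher after a delay.
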(event `self.ReceiveBeginPlay`
  ;[1 1 1] Attach weapon
  (bind _returnvalue (`|SpawnActorFromClass` "/Game/Blueprints/Rifle.Rifle_C" (`self.GetTransform`) "AlwaysSpawn" "OverrideRootScale" null null))
  (`self.K2_AttachRootComponentTo` _returnvalue (`SceneComponent.GetChildComponent` (`self.K2_GetRootComponent`) 1) "WeaponPoint" "SnapToTarget" true)
  ;[1 1 1] Hear Noise
  (add `PawnSensingComponent.OnHearNoise` (`self.PawnSensing1`) (delegate `OnHearNoise_Event`)))

(event `OnHearNoise_Event`
  (params (Instigator :type "Pawn Object Reference") (Location :type "Vector Structure (by ref)") (Volume :type "Float (double-precision)"))
  ;[1 1 1] Hear Noise
)

(event `EnemyFound_Event`
  ;[1 1 1] Spawn Projectile - Firing
  (set `self.Attacking` true)
  (`/Engine/EditorBlueprintResources/StandardMacros.DoOnce` false :!label _label
    (:`Completed`
      (`|SpawnActorFromClass` "/Game/Blueprints/BotProjectile.BotProjectile_C" (`KismetMathLibrary.MakeTransform` (.location (`self.GetTransform` (stale `self.ReceiveBeginPlay` _returnvalue))) (`KismetMathLibrary.MakeRotator` (.roll (.rotation (`self.GetTransform` (stale `self.ReceiveBeginPlay` _returnvalue)))) (.pitch (.rotation (`self.GetTransform` (stale `self.ReceiveBeginPlay` _returnvalue)))) (+ (.yaw (.rotation (`self.GetTransform` (stale `self.ReceiveBeginPlay` _returnvalue)))) 90.0)) (.scale (`self.GetTransform` (stale `self.ReceiveBeginPlay` _returnvalue)))) "AlwaysSpawn" "OverrideRootScale" null null)
      (`GameplayStatics.SpawnSoundAttached` "/Game/Audio/OLD/Template1rst_WeaponFire02.Template1rst_WeaponFire02" (`self.K2_GetRootComponent`) "None" (0.0 0.0 0.0) (struct) "KeepRelativeOffset" false 1.0 1.0 0.0 null null)
      (`KismetSystemLibrary.Delay` 0.2)
      (goto _label :!via `Reset`))))

(event `BotDeath_Event`
  ;[1 1 1] Death
  (set `self.Alive` false)
  (`SkeletalMeshComponent.PlayAnimation` (`self.Mesh`) "/Game/Animations/TTP_Animations/Death.Death" false)
  (`KismetSystemLibrary.Delay` 1.5)
  (`self.BotHasDied`))

(fn `UserConstructionScript`)